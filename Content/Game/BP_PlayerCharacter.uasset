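; Player character Blueprint that reports hits on its HealthComponent as game messages, with no other active logic in its graphs.
; Two identical HitSig handlers each look up the FSDGameState through GetAllActorsOfClass and call PostGameMessage on the first result.
; The message concatenates damage amount, damage class name, causer name and the AnyHealthLost flag.
; BeginPlay, overlap, Tick and the construction script are empty.
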(fn `BndEvt__HealthComponent_K2Node_ComponentBoundEvent_0_HitSig__DelegateSignature`
  (params (Damage :type "Float (double-precision)") (DamageClass :type "DamageClass Object Reference (by ref)") (DamageCauser :type "Actor Object Reference (by ref)") (anyHealthLost :type "Boolean (by ref)"))
  (bind _outactors (`GameplayStatics.GetAllActorsOfClass` "/Script/FSD.FSDGameState"))
  (`FSDGameState.PostGameMessage` (`|GetArrayItem` _outactors) (`KismetStringLibrary.Concat_StrStr` (`KismetStringLibrary.Conv_DoubleToString` Damage) " " (`KismetSystemLibrary.GetDisplayName` DamageClass) " " (`KismetSystemLibrary.GetDisplayName` DamageCauser) "" (`KismetStringLibrary.Conv_BoolToString` anyHealthLost))))

(fn `BndEvt__HealthComponent_K2Node_ComponentBoundEvent_1_HitSig__DelegateSignature`
  (params (Damage :type "Float (double-precision)") (DamageClass :type "DamageClass Object Reference (by ref)") (DamageCauser :type "Actor Object Reference (by ref)") (anyHealthLost :type "Boolean (by ref)"))
  (bind _outactors (`GameplayStatics.GetAllActorsOfClass` "/Script/FSD.FSDGameState"))
  (`FSDGameState.PostGameMessage` (`|GetArrayItem` _outactors) (`KismetStringLibrary.Concat_StrStr` (`KismetStringLibrary.Conv_DoubleToString` Damage) " " (`KismetSystemLibrary.GetDisplayName` DamageClass) " " (`KismetSystemLibrary.GetDisplayName` DamageCauser) "" (`KismetStringLibrary.Conv_BoolToString` anyHealthLost))))

(fn `UserConstructionScript`)