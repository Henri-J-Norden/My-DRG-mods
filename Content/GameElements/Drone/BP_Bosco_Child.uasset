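; BP_Bosco_Child is a child Blueprint of the Bosco drone that reports drone events as game messages.
; Its construction script runs the parent's, then caches the FSD game state.
; Handlers for revive use, player salute and state change post the remaining revive charges, a salute notice or the current state through that game state.
; SelfDestruct has an empty body, and the event graph holds only disabled stubs.
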(fn `On Player Salute`
  (params (`Player Character` :type "PlayerCharacter Object Reference"))
  (`/Game/_ModBPs/MyMods/_/GlobalFunctionsGlosb.Post Multiline Game Message` (`KismetStringLibrary.Concat_StrStr` "Player saluted") (`self.FSDGameState`)))

(fn `On Revive Used`
  (bind _returnvalue (`Bosco.GetReviveCharges`))
  (`/Game/_ModBPs/MyMods/_/GlobalFunctionsGlosb.Post Multiline Game Message` (`KismetStringLibrary.Concat_StrStr` "Bosco revives: " (`KismetStringLibrary.Conv_IntToString` _returnvalue)) (`self.FSDGameState`)))

(fn `On State Changed`
  (bind _returnvalue (`Bosco.GetCurrentState`))
  (`/Game/_ModBPs/MyMods/_/GlobalFunctionsGlosb.Post Multiline Game Message` (`KismetStringLibrary.Concat_StrStr` "Bosco state: " (`|GetEnumeratorNameAsString` _returnvalue)) (`self.FSDGameState`)))

(fn `SelfDestruct`)

(fn `UserConstructionScript`
  (`parent.UserConstructionScript`)
  (bind _fsd_game_state (`/Game/_ModBPs/MyMods/_/GlobalFunctionsGlosb.Get FSD Game State`))
  (set `self.FSDGameState` _fsd_game_state))